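; Spike trap actor that flashes a warning plane with a click when its trigger box is overlapped, then raises three spikes and lowers them after a short hold.
; SpikeOn and SpikeOff offset each spike vertically and set the TrapTriggered guard.
; HitBox overlaps call the game mode's spike trap dispatcher through a DoOnce, reset after retraction.
; At BeginPlay it registers DestroyTrap with the game mode as its disabler.
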(event `self.ReceiveBeginPlay`
  (`SceneComponent.SetVisibility` (`self.Plane`) false false)
  (bind _asbp_gamemode (cast `/Game/LABWORK1/BP_Gamemode` (`GameplayStatics.GetGameMode`)))
  (bind _output_get (set `self.GamemodeRef` _asbp_gamemode))
  (add `/Game/LABWORK1/BP_Gamemode.SpikeTrapDisabler` _output_get (delegate `Destroy Trap`)))

(event `Destroy Trap`
  (`self.K2_DestroyActor`))

(event `self.TriggerBox.OnComponentBeginOverlap`
  (params (OverlappedComponent :type "PrimitiveComponent Object Reference") (OtherActor :type "Actor Object Reference") (OtherComp :type "PrimitiveComponent Object Reference") (OtherBodyIndex :type Integer) (bFromSweep :type Boolean) (SweepResult :type "HitResult Structure (by ref)"))
  (if (not (`self.TrapTriggered`))
    (`SceneComponent.SetVisibility` (`self.Plane`) true false)
    (`GameplayStatics.PlaySoundAtLocation` "/Engine/VREditor/Sounds/UI/Click_on_Button.Click_on_Button" (0.0 0.0 0.0) (struct) 1.0 1.0 0.0 null null null null)
    (`KismetSystemLibrary.Delay` 0.35)
    (`SceneComponent.SetVisibility` (`self.Plane`) false false)
    (`self.SpikeOn` (`self.Spike`)
      (:`ExecOut`
        (`self.SpikeOn` (`self.Spike1`)
          (:`ExecOut`
            (`self.SpikeOn` (`self.Spike2`)
              (:`ExecOut`
                (`KismetSystemLibrary.Delay` 2.0)
                (`GameplayStatics.PlaySoundAtLocation` "/Engine/VREditor/Sounds/UI/Click_on_Button.Click_on_Button" (0.0 0.0 0.0) (struct) 1.0 1.0 0.0 null null null null)
                (`self.SpikeOff` (`self.Spike`)
                  (:`ExecOut`
                    (`self.SpikeOff` (`self.Spike1`)
                      (:`ExecOut`
                        (`self.SpikeOff` (`self.Spike2`)
                          (:`ExecOut`
                            (goto _label :!via `Reset`)))))))))))))))

(event `self.HitBox.OnComponentBeginOverlap`
  (params (OverlappedComponent :type "PrimitiveComponent Object Reference") (OtherActor :type "Actor Object Reference") (OtherComp :type "PrimitiveComponent Object Reference") (OtherBodyIndex :type Integer) (bFromSweep :type Boolean) (SweepResult :type "HitResult Structure (by ref)"))
  (`/Engine/EditorBlueprintResources/StandardMacros.DoOnce` false :!label _label
    (:`Completed`
      (`/Game/LABWORK1/BP_Gamemode.SpikeTrapDispatcher` (`self.GamemodeRef`)))))

(fn `UserConstructionScript`)