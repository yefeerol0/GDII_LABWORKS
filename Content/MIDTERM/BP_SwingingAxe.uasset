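; BP_SwingingAxe is a swinging axe trap driven by BP_Gamemode dispatchers, bound on BeginPlay.
; The trigger dispatcher plays the Swinging timeline if WireConnected is true, adding a scaled track value to the actor's current pitch each update.
; Axe hits call the gamemode's hit dispatcher, throttled by a DoOnce that resets after a short delay.
; The disabler dispatcher destroys the actor.
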(event `Axe Disabler`
  (`self.K2_DestroyActor`))

(event `self.ReceiveBeginPlay`
  (bind _asbp_gamemode (cast `/Game/LABWORK1/BP_Gamemode` (`GameplayStatics.GetGameMode`)))
  (bind _output_get (set `self.GamemodeRef` _asbp_gamemode))
  (add `/Game/LABWORK1/BP_Gamemode.SwingingAxeTriggerDispatcher` _output_get (delegate `SwingingMovement`))
  (add `/Game/LABWORK1/BP_Gamemode.AxeTrapDisabler` _output_get (delegate `Axe Disabler`)))

(event `SwingingMovement`
  (bind (_returnvalue_roll _returnvalue_pitch _returnvalue_yaw) (`KismetMathLibrary.BreakRotator` (`self.K2_GetActorRotation`)))
  (if (`self.wireConnected`)
    (bind (_direction _123) (`Timeline|Swinging`)
      (:`Update`
        (`self.K2_SetActorRotation` (`KismetMathLibrary.MakeRotator` 0.0 (+ (* _123 1.2) _returnvalue_pitch) _returnvalue_yaw))))))

(event `self.Axe.OnComponentHit`
  (params (HitComponent :type "PrimitiveComponent Object Reference") (OtherActor :type "Actor Object Reference") (OtherComp :type "PrimitiveComponent Object Reference") (NormalImpulse :type "Vector Structure") (Hit :type "HitResult Structure (by ref)"))
  (`/Engine/EditorBlueprintResources/StandardMacros.DoOnce` false :!label _label
    (:`Completed`
      (`/Game/LABWORK1/BP_Gamemode.SwingingAxeHitDispatcher` (`self.GamemodeRef`))
      (`KismetSystemLibrary.Delay` 3.0)
      (goto _label :!via `Reset`))))

(fn `UserConstructionScript`)