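; Trigger actor that sets off swinging axes through the game mode when any actor overlaps it.
; On BeginPlay it caches BP_Gamemode and flags three referenced swinging axes as wire-connected.
; On overlap it calls the game mode's swinging axe trigger dispatcher rather than calling the axes directly, with no filter on the overlapping actor.
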(event `self.ReceiveBeginPlay`
  (bind _asbp_gamemode (cast `/Game/LABWORK1/BP_Gamemode` (`GameplayStatics.GetGameMode`)))
  (set `self.GamemodeRef` _asbp_gamemode)
  (set `/Game/LABWORK1/BP_SwingingAxe.wireConnected` true (`self.SwingingAxeRef1`))
  (set `/Game/LABWORK1/BP_SwingingAxe.wireConnected` true (`self.SwingingAxeRef2`))
  (set `/Game/LABWORK1/BP_SwingingAxe.wireConnected` true (`self.SwingingAxeRef3`)))

(event `self.ReceiveActorBeginOverlap`
  (params (OtherActor :type "Actor Object Reference"))
  (`/Game/LABWORK1/BP_Gamemode.SwingingAxeTriggerDispatcher` (`self.GamemodeRef`)))

(fn `UserConstructionScript`)