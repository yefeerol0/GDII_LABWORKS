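; BP_PoisonousGas is a poison gas trap that slows the player and flags poison exposure in the gamemode.
; It caches BP_Gamemode and player character on BeginPlay and binds DisableTrap to the gamemode's PoisonTrapDisabler event, destroying itself.
; Actor overlap sets InPoisonArea, fires the poison dispatcher and lowers walk speed.
; Ending Gas component overlap clears the flag and sets a faster speed, neither handler checking the overlapping actor.
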(event `self.ReceiveBeginPlay`
  (bind _asbp_gamemode (cast `/Game/LABWORK1/BP_Gamemode` (`GameplayStatics.GetGameMode`)))
  (bind _output_get (set `self.GamemodeRef` _asbp_gamemode))
  (bind _asbp_third_person_character (cast `/Game/LABWORK1/BP_ThirdPersonCharacter` (`GameplayStatics.GetPlayerCharacter` 0)))
  (set `self.PlayerCharRef` _asbp_third_person_character)
  (add `/Game/LABWORK1/BP_Gamemode.PoisonTrapDisabler` _output_get (delegate `DisableTrap`)))

(event `self.ReceiveActorBeginOverlap`
  (params (OtherActor :type "Actor Object Reference"))
  (bind _gamemoderef (`self.GamemodeRef`))
  (set `/Game/LABWORK1/BP_Gamemode.InPoisonArea` true _gamemoderef)
  (`/Game/LABWORK1/BP_Gamemode.PoisonDispatcher` _gamemoderef)
  (set `CharacterMovementComponent.MaxWalkSpeed` 150.0 (`Character.CharacterMovement` (`self.PlayerCharRef`))))

(event `DisableTrap`
  (`self.K2_DestroyActor`))

(event `self.Gas.OnComponentEndOverlap`
  (params (OverlappedComponent :type "PrimitiveComponent Object Reference") (OtherActor :type "Actor Object Reference") (OtherComp :type "PrimitiveComponent Object Reference") (OtherBodyIndex :type Integer))
  (set `/Game/LABWORK1/BP_Gamemode.InPoisonArea` false (`self.GamemodeRef`))
  (set `CharacterMovementComponent.MaxWalkSpeed` 500.0 (`Character.CharacterMovement` (`self.PlayerCharRef`))))

(fn `UserConstructionScript`)