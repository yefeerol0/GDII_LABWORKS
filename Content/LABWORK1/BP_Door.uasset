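; BP_Door is an interactable sliding door that opens only when the game mode's Keys value exactly equals the door's KeyNumber.
; It caches BP_Gamemode on BeginPlay, and Interact either plays the DoorOpen timeline or prints a wrong-key message.
; The timeline lerps the Door component's relative location from StartLocation to FinishLocation without sweep.
; The construction script applies the Material variable to the door.
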(event `self.ReceiveBeginPlay`
  (bind _asbp_gamemode (cast `/Game/LABWORK1/BP_Gamemode` (`GameplayStatics.GetGameMode`)))
  (set `self.GamemodeRef` _asbp_gamemode))

(event `/Game/LABWORK1/BPI_Interact.Interact`
  (if (== (`/Game/LABWORK1/BP_Gamemode.Keys` (`self.GamemodeRef`)) (`self.KeyNumber`))
    (bind (_direction _newtrack_0) (`Timeline|DoorOpen`)
      (:`Update`
        (`SceneComponent.K2_SetRelativeLocation` (`self.Door`) (`KismetMathLibrary.VLerp` (`self.StartLocation`) (`self.FinishLocation`) _newtrack_0) false false)))
    (else
      (`KismetSystemLibrary.PrintString` "You do not have the correct key!"))))

(fn `UserConstructionScript`
  (`PrimitiveComponent.SetMaterial` (`self.Door`) 0 (`self.Material`)))