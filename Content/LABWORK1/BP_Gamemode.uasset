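; BP_Gamemode is a game mode that creates the HUD and runs a countdown with a win condition.
; An enter dispatcher starts the countdown and an exit dispatcher sets the win flag, each handler unbinding after its first call.
; A looping one-second timer decrements Timer while active; otherwise, including before the start, it calls a light dispatcher each tick with Timer and WinCondition.
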(event `TimerStart`
  (set `self.TimerStarted` true)
  (remove `self.EnterDispatcher` (delegate `TimerStart`)))

(event `self.ReceiveBeginPlay`
  (bind _returnvalue (`|GenericCreateObject` "/Game/LABWORK1/BP_HUD.BP_HUD_C"))
  (`UserWidget.AddToViewport` _returnvalue 0)
  (`KismetSystemLibrary.K2_SetTimerDelegate` (delegate `TimerEvent`) 1.0 true)
  (add `self.ExitDispatcher` (delegate `TimerStop`))
  (add `self.EnterDispatcher` (delegate `TimerStart`)))

(event `TimerEvent`
  (if (and (!= (`self.Timer`) 0) (!= (`self.WinCondition`) true) (`self.TimerStarted`))
    (bind _output_get (set `self.Timer` (- (`self.Timer`) 1)))
    (else
      (`self.LightDispatcher` _output_get (`self.WinCondition`)))))

(event `TimerStop`
  (set `self.WinCondition` true)
  (remove `self.ExitDispatcher` (delegate `TimerStop`)))

(fn `UserConstructionScript`)