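; BP_Key is an interactable key pickup that records its key number in BP_Gamemode.
; On BeginPlay it caches the game mode through a cast.
; Interact overwrites the game mode's Keys value with this key's KeyNumber, prints an acquired message using the matching Names entry, then destroys the actor.
; The construction script applies the Material variable to the Key component, allowing a different look per instance.
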(event `self.ReceiveBeginPlay`
  (bind _asbp_gamemode (cast `/Game/LABWORK1/BP_Gamemode` (`GameplayStatics.GetGameMode`)))
  (set `self.GMReference` _asbp_gamemode))

(event `/Game/LABWORK1/BPI_Interact.Interact`
  (bind _output_get (set `/Game/LABWORK1/BP_Gamemode.Keys` (`self.KeyNumber`) (`self.GMReference`)))
  (`KismetSystemLibrary.PrintString` (`KismetStringLibrary.Concat_StrStr` "Key " (`|GetArrayItem` (`self.Names`) _output_get) " " "Acquired"))
  (`self.K2_DestroyActor`))

(fn `UserConstructionScript`
  (`PrimitiveComponent.SetMaterial` (`self.Key`) 0 (`self.Material`)))