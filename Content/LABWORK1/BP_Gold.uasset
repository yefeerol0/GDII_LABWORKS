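; BP_Gold is a gold pickup worth a random amount.
; On BeginPlay it rolls its value, caches BP_Gamemode and hides extra cone meshes so the pile size reflects the value.
; Interact adds the value to the game mode's GoldCollected, prints the gain and total, then destroys the actor.
; An unconnected Construction Script branch that would add the gold meshes dynamically never runs.
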(event `self.ReceiveBeginPlay`
  (set `self.RandomValue` (`KismetMathLibrary.RandomIntegerInRange` 1 99))
  (bind _asbp_gamemode (cast `/Game/LABWORK1/BP_Gamemode` (`GameplayStatics.GetGameMode`)))
  (set `self.Gamemode_Ref` _asbp_gamemode)
  (if (<= (`self.RandomValue`) 25)
    (`SceneComponent.SetVisibility` (`self.Cone2`) false false)
    (`SceneComponent.SetVisibility` (`self.Cone3`) false false)
    (elif (<= (`self.RandomValue`) 75)
      (`SceneComponent.SetVisibility` (`self.Cone3`) false false))))

(event `/Game/LABWORK1/BPI_Interact.Interact`
  (bind _gamemode_ref (`self.Gamemode_Ref`))
  (bind _output_get (set `/Game/LABWORK1/BP_Gamemode.GoldCollected` (+ (`/Game/LABWORK1/BP_Gamemode.GoldCollected` _gamemode_ref) (`self.RandomValue`)) _gamemode_ref))
  (`KismetSystemLibrary.PrintString` (`KismetStringLibrary.Concat_StrStr` (`KismetStringLibrary.Conv_IntToString` (`self.RandomValue`)) " gold collected!" " Total gold: " (`KismetStringLibrary.Conv_IntToString` _output_get)))
  (`self.K2_DestroyActor`))

(fn `UserConstructionScript`)