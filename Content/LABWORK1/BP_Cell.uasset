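; BP_Cell is a modular grid room cell whose light signals win or lose state during play.
; The construction script scales the floor from GridSize and adds optional walls, a ceiling and, under a ceiling, a point light.
; At BeginPlay it binds to the game mode's light dispatcher, turning the light red and calling the lose dispatcher when the timer hits zero, or green on a win.
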(event `self.ReceiveBeginPlay`
  (bind _asbp_gamemode (cast `/Game/LABWORK1/BP_Gamemode` (`GameplayStatics.GetGameMode`)))
  (bind _output_get (set `self.GamemodeRef` _asbp_gamemode))
  (add `/Game/LABWORK1/BP_Gamemode.LightDispatcher` _output_get (delegate `SwitchLightColor`)))

(event `SwitchLightColor`
  (params (TimerCheck :type Integer) (WinConditionCheck :type Boolean))
  (if (== TimerCheck 0)
    (`LightComponent.SetLightColor` (`self.GetComponentByClass` "/Script/Engine.PointLightComponent") (struct :`R` 1.0 :`A` 1.0) true)
    (`/Game/LABWORK1/BP_Gamemode.LoseDispatcher` (`self.GamemodeRef`))
    (elif WinConditionCheck
      (`LightComponent.SetLightColor` (`self.GetComponentByClass` "/Script/Engine.PointLightComponent") (struct :`R` 0.001014 :`G` 1.0 :`A` 1.0) true))))

(fn `UserConstructionScript`
  (locals (WallThickness :type "Float (double-precision)") (WallLenght :type "Float (double-precision)"))
  (bind _gridsize (`self.GridSize`))
  (bind _walllenght (`local.WallLenght`))
  (bind _walllenght_2 (`local.WallLenght`))
  (bind _returnvalue (* (`local.WallLenght`) 0.5))
  (set `local.WallLenght` _gridsize)
  (set `local.WallThickness` (* _gridsize 0.1))
  (`SceneComponent.SetRelativeScale3D` (`self.Floor`) (`self.SizeToCube` (`KismetMathLibrary.MakeVector` _walllenght _walllenght (`local.WallThickness`))))
  (if (`self.WestWall`)
    (`AddComponent|NODE_AddStaticMeshComponent-0` :`RelativeTransform` (`KismetMathLibrary.MakeTransform` (0.0 0.0 0.0) (struct) (`self.SizeToCube` (`KismetMathLibrary.MakeVector` (`local.WallLenght`) (`local.WallThickness`) (`self.WallHeight`))))))
  (if (`self.SouthWall`)
    (`AddComponent|NODE_AddStaticMeshComponent-1` :`RelativeTransform` (`KismetMathLibrary.MakeTransform` (0.0 0.0 0.0) (struct) (`self.SizeToCube` (`KismetMathLibrary.MakeVector` (`local.WallThickness`) (`local.WallLenght`) (`self.WallHeight`))))))
  (if (`self.NorthWall`)
    (`AddComponent|NODE_AddStaticMeshComponent-2` :`RelativeTransform` (`KismetMathLibrary.MakeTransform` (`KismetMathLibrary.MakeVector` (- (`local.WallLenght`) (`local.WallThickness`))) (struct) (`self.SizeToCube` (`KismetMathLibrary.MakeVector` (`local.WallThickness`) (`local.WallLenght`) (`self.WallHeight`))))))
  (if (`self.EastWall`)
    (`AddComponent|NODE_AddStaticMeshComponent-3` :`RelativeTransform` (`KismetMathLibrary.MakeTransform` (`KismetMathLibrary.MakeVector` 0.0 (- (`local.WallLenght`) (`local.WallThickness`))) (struct) (`self.SizeToCube` (`KismetMathLibrary.MakeVector` (`local.WallLenght`) (`local.WallThickness`) (`self.WallHeight`))))))
  (if (`self.Ceiling`)
    (`AddComponent|NODE_AddStaticMeshComponent-4` :`RelativeTransform` (`KismetMathLibrary.MakeTransform` (`KismetMathLibrary.MakeVector` 0.0 0.0 (`self.WallHeight`)) (struct) (`self.SizeToCube` (`KismetMathLibrary.MakeVector` _walllenght_2 _walllenght_2 (`local.WallThickness`)))))
    (if (> (`self.LightIntensity`) 0.0)
      (bind _returnvalue_2 (`AddComponent|NODE_AddPointLightComponent-0` :`RelativeTransform` (`KismetMathLibrary.MakeTransform` (`KismetMathLibrary.MakeVector` _returnvalue _returnvalue (* (`self.WallHeight`) 0.8)))))
      (`LightComponent.SetLightColor` _returnvalue_2 (`self.LightColor`) true)
      (`LightComponent.SetIntensity` _returnvalue_2 (`self.LightIntensity`)))))